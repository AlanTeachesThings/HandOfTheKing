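; Game mode for a Hand of the King card game, running turn-based play on a card grid and declaring a winner.
; Startup builds the grid, HUD, house banners and 1-indexed players with active and inactive widgets.
; While executing, Tick polls cards until idle, then rotates players or ends the game when Varys's row and column hold no eligible cards.
; Banners pass to players matching or beating the owner's house count; most banners wins.
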(event `self.ReceiveBeginPlay`
  (bind (_output_number _output_name _output_activewidget) (break `/Game/Player` (`|GetArrayItem` (`self.Players`) 1)))
  (bind _outactors (`GameplayStatics.GetAllActorsOfClass` "/Script/Engine.CameraActor"))
  (`PlayerController.SetViewTargetWithBlend` (`GameplayStatics.GetPlayerController` 0) (`|GetArrayItem` _outactors) 0.0 "VTBlend_Linear" 0.0 false)
  (bind _outactors_2 (`GameplayStatics.GetAllActorsOfClass` "/Game/Cards/Grid_A.Grid_A_C"))
  (bind _output_get (set `self.Grid` (`|GetArrayItem` _outactors_2)))
  (`/Game/Cards/Grid_A.CreateCards` _output_get)
  (bind _returnvalue (`|CreateWidget` "/Game/UI/GameHUD.GameHUD_C"))
  (bind _output_get_2 (set `self.HUDReference` _returnvalue))
  (`UserWidget.AddToViewport` _output_get_2 0)
  (set `self.UnclaimedBanners` (`/Game/UI/GameHUD.UnclaimedBanners` _output_get_2))
  (`self.CreateBanners`)
  (`self.CreatePlayers`)
  (`/Game/UI/ActivePlayerUI.Reveal` _output_activewidget)
  (`self.WaitForInput`))

(event `WaitForInput`
  (bind _returnvalue (`GameplayStatics.GetPlayerController` 0))
  (set `PlayerController.bShowMouseCursor` true _returnvalue)
  (set `PlayerController.bEnableMouseOverEvents` true _returnvalue)
  (set `PlayerController.bEnableClickEvents` true _returnvalue)
  (set `self.GameStatus` "NewEnumerator0"))

(event `WaitForExecutionsToFinish`
  (bind _returnvalue (`GameplayStatics.GetPlayerController` 0))
  (set `PlayerController.bShowMouseCursor` false _returnvalue)
  (set `PlayerController.bEnableMouseOverEvents` false _returnvalue)
  (set `PlayerController.bEnableClickEvents` false _returnvalue)
  (set `self.GameStatus` "NewEnumerator1"))

(event `self.ReceiveTick`
  (params (DeltaSeconds :type "Float (single-precision)"))
  (bind _returnvalue (`GameplayStatics.GetPlayerController` 0))
  (bind (_output_number _output_name _output_activewidget) (break `/Game/Player` (`|GetArrayItem` (`self.Players`) (`self.CurrentPlayer`))))
  (bind (_output_number_2 _output_name_2 _output_activewidget_2) (break `/Game/Player` (`|GetArrayItem` (`self.Players`) (`self.CurrentPlayer`))))
  (switch `/Game/GameStatus` (`self.GameStatus`)
    (:`NewEnumerator1`
      (bind _ready (`self.CheckForExecutions`))
      (if _ready
        (bind (_gameend _winningplayer) (`self.CheckForGameEnd`))
        (if _gameend
          (bind _returnvalue_2 (`|CreateWidget` "/Game/UI/GameOver_UI.GameOver_UI_C" null _winningplayer))
          (`UserWidget.AddToViewport` _returnvalue_2 0)
          (set `PlayerController.bShowMouseCursor` true _returnvalue)
          (set `PlayerController.bEnableMouseOverEvents` true _returnvalue)
          (set `PlayerController.bEnableClickEvents` true _returnvalue)
          (else
            ;[1 1 1] Executions are done - check for next player, then wait for input
            (`/Game/UI/ActivePlayerUI.Hide` _output_activewidget)
            (bind _output_get (set `self.CurrentPlayer` (+ (`self.CurrentPlayer`) 1)))
            (if (> _output_get (`self.NumberOfPlayers`))
              (set `self.CurrentPlayer` 1))
            (`/Game/UI/ActivePlayerUI.Reveal` _output_activewidget_2)
            (`self.WaitForInput`)))))))

(event `CheckBanners`)

(fn `CheckForExecutions`
  (returns (Ready :type Boolean))
  (locals (ReadyToContinue :type Boolean :default true))
  (set `local.ReadyToContinue` true)
  (bind _outactors (`GameplayStatics.GetAllActorsOfClass` "/Game/Cards/Card_A.Card_A_C"))
  (for _array_element _outactors
    (if (`/Game/Cards/Card_A.ExecutingActions` _array_element)
      (set `local.ReadyToContinue` false)))
  (return (`local.ReadyToContinue`)))

(fn `CheckForGameEnd`
  (returns (GameEnd :type Boolean) (WinningPlayer :type Integer))
  (locals (GameEnding :type Boolean :default true) (CurrentWinner :type Integer) (HighestBannerCount :type Integer) (BannersCounted :type Integer))
  (bind _grid (`self.Grid`))
  (bind _gameending (`local.GameEnding`))
  (set `local.GameEnding` true)
  (bind _varysposition (`/Game/Cards/Grid_A.FindVarys` _grid))
  (bind _values (`BlueprintMapLibrary.Map_Values` (`/Game/Cards/Grid_A.Cards` _grid)))
  (for _array_element _values
    (`/Engine/EditorBlueprintResources/StandardMacros.IsValid` _array_element
      (:`Is Valid`
        (bind (_carddata_cardname _carddata_cardhouse) (break `/Game/Cards/CardData_Struct` (`/Game/Cards/Card_A.CardData` _array_element)))
        (if (`|EnumInequality` _carddata_cardhouse "NewEnumerator7")
          (bind (_x _y) (`KismetMathLibrary.BreakVector2D` _varysposition))
          (bind (_gridposition_x _gridposition_y) (`KismetMathLibrary.BreakVector2D` (`/Game/Cards/Card_A.GridPosition` _array_element)))
          (if (or (== _x _gridposition_x) (== _y _gridposition_y))
            (set `local.GameEnding` false))))))
  (if _gameending
    (set `local.CurrentWinner` 0)
    (set `local.HighestBannerCount` 0)
    (for _array_element_2 (`self.Players`)
      (set `local.BannersCounted` 0)
      (bind _values_2 (`BlueprintMapLibrary.Map_Values` (`self.BannerOwners`)))
      (for _array_element_3 _values_2
        (if (== (break `/Game/Player` _array_element_2) _array_element_3)
          (set `local.BannersCounted` (+ (`local.BannersCounted`) 1))))
      (if (> (`local.BannersCounted`) (`local.HighestBannerCount`))
        (set `local.CurrentWinner` (break `/Game/Player` _array_element_2))
        (set `local.HighestBannerCount` (`local.BannersCounted`))))
    (return (`local.GameEnding`) (`local.CurrentWinner`))
    (else
      (return _gameending 0))))

(fn `CreateBanners`
  (bind _bannerowners (`self.BannerOwners`))
  (bind _bannerwidgets (`self.BannerWidgets`))
  (bind _bannercontainer (`/Game/UI/UnclaimedBanners.BannerContainer` (`self.UnclaimedBanners`)))
  (`|ExecutionSequence`
    (:`then_0`
      (bind _returnvalue (`|CreateWidget` "/Game/UI/Banner.Banner_C"))
      (`BlueprintMapLibrary.Map_Add` _bannerwidgets "NewEnumerator0" _returnvalue)
      (`HorizontalBox.AddChildToHorizontalBox` _bannercontainer _returnvalue)
      (`BlueprintMapLibrary.Map_Add` _bannerowners "NewEnumerator0"))
    (:`then_1`
      (bind _returnvalue_2 (`|CreateWidget` "/Game/UI/Banner.Banner_C" null "NewEnumerator1"))
      (`BlueprintMapLibrary.Map_Add` _bannerwidgets "NewEnumerator1" _returnvalue_2)
      (`HorizontalBox.AddChildToHorizontalBox` _bannercontainer _returnvalue_2)
      (`BlueprintMapLibrary.Map_Add` _bannerowners "NewEnumerator1"))
    (:`then_2`
      (bind _returnvalue_3 (`|CreateWidget` "/Game/UI/Banner.Banner_C" null "NewEnumerator2"))
      (`BlueprintMapLibrary.Map_Add` _bannerwidgets "NewEnumerator2" _returnvalue_3)
      (`HorizontalBox.AddChildToHorizontalBox` _bannercontainer _returnvalue_3)
      (`BlueprintMapLibrary.Map_Add` _bannerowners "NewEnumerator2"))
    (:`then_3`
      (bind _returnvalue_4 (`|CreateWidget` "/Game/UI/Banner.Banner_C" null "NewEnumerator3"))
      (`BlueprintMapLibrary.Map_Add` _bannerwidgets "NewEnumerator3" _returnvalue_4)
      (`HorizontalBox.AddChildToHorizontalBox` _bannercontainer _returnvalue_4)
      (`BlueprintMapLibrary.Map_Add` _bannerowners "NewEnumerator3"))
    (:`then_4`
      (bind _returnvalue_5 (`|CreateWidget` "/Game/UI/Banner.Banner_C" null "NewEnumerator4"))
      (`BlueprintMapLibrary.Map_Add` _bannerwidgets "NewEnumerator4" _returnvalue_5)
      (`HorizontalBox.AddChildToHorizontalBox` _bannercontainer _returnvalue_5)
      (`BlueprintMapLibrary.Map_Add` _bannerowners "NewEnumerator4"))
    (:`then_5`
      (bind _returnvalue_6 (`|CreateWidget` "/Game/UI/Banner.Banner_C" null "NewEnumerator5"))
      (`BlueprintMapLibrary.Map_Add` _bannerwidgets "NewEnumerator5" _returnvalue_6)
      (`HorizontalBox.AddChildToHorizontalBox` _bannercontainer _returnvalue_6)
      (`BlueprintMapLibrary.Map_Add` _bannerowners "NewEnumerator5"))
    (:`then_6`
      (bind _returnvalue_7 (`|CreateWidget` "/Game/UI/Banner.Banner_C" null "NewEnumerator6"))
      (`BlueprintMapLibrary.Map_Add` _bannerwidgets "NewEnumerator6" _returnvalue_7)
      (`HorizontalBox.AddChildToHorizontalBox` _bannercontainer _returnvalue_7)
      (`BlueprintMapLibrary.Map_Add` _bannerowners "NewEnumerator6"))))

(fn `CreatePlayers`
  (`KismetArrayLibrary.Array_Add` (`self.Players`)) ; I don't care what anyone says,\nI'm indexing my players from 1!
  (for _index (range 1 (+ (`self.NumberOfPlayers`) 1))
    (bind _returnvalue (`|CreateWidget` "/Game/UI/ActivePlayerUI.ActivePlayerUI_C" null _index))
    (`/Game/UI/ActivePlayerUI.Hide` _returnvalue)
    (`UserWidget.AddToViewport` _returnvalue 0)
    (bind _returnvalue_2 (`|CreateWidget` "/Game/UI/InactivePlayerUI.InactivePlayerUI_C" null _index))
    (`PanelWidget.AddChild` (`/Game/UI/GameHUD.InactivePlayerWidgets` (`self.HUDReference`)) _returnvalue_2)
    (`BlueprintMapLibrary.Map_Add` (`self.InactivePlayerWidgets`) _index _returnvalue_2)
    (bind _player (make `/Game/Player` _index "" _returnvalue (`|MakeMap` "NewEnumerator0" 0 "NewEnumerator1" 0 "NewEnumerator2" 0 "NewEnumerator3" 0 "NewEnumerator4" 0 "NewEnumerator5" 0 "NewEnumerator6" :!type "/Game/Cards/House_Enum Enum")))
    (`KismetArrayLibrary.Array_Insert` (`self.Players`) _player _index)
    (`/Game/UI/ActivePlayerUI.UpdateCardCount` _returnvalue _player)
    (`/Game/UI/InactivePlayerUI.UpdateCardCount` _returnvalue_2 _player)
    (`/Game/UI/InactivePlayerUI.UpdateBanners` _returnvalue_2)))

(fn `UpdateBanners`
  (params (HouseToCheck :type "/Game/Cards/House_Enum Enum" :default "NewEnumerator0"))
  (bind _currentplayer (`self.CurrentPlayer`))
  (bind _players (`self.Players`))
  (bind _value (`BlueprintMapLibrary.Map_Find` (`self.BannerWidgets`) HouseToCheck))
  (bind _value_2 (`BlueprintMapLibrary.Map_Find` (`self.BannerOwners`) HouseToCheck))
  (bind (_output_number _output_name _output_activewidget _output_cardstaken) (break `/Game/Player` (`|GetArrayItem` _players _currentplayer)))
  (bind (_output_number_2 _output_name_2 _output_activewidget_2 _output_cardstaken_2) (break `/Game/Player` (`|GetArrayItem` _players _value_2)))
  (if (!= _currentplayer _value_2)
    (if (>= (`BlueprintMapLibrary.Map_Find` _output_cardstaken HouseToCheck) (`BlueprintMapLibrary.Map_Find` _output_cardstaken_2 HouseToCheck))
      (`BlueprintMapLibrary.Map_Add` (`self.BannerOwners`) HouseToCheck _currentplayer)
      (`Widget.RemoveFromParent` _value)
      (`HorizontalBox.AddChildToHorizontalBox` (`/Game/UI/ActivePlayerUI.BannerContainer` _output_activewidget_2) _value))))

(fn `UpdateUI`
  (bind _inactiveplayerwidgets (`self.InactivePlayerWidgets`))
  (bind _keys (`BlueprintMapLibrary.Map_Keys` _inactiveplayerwidgets))
  (for _array_element _keys
    (bind _value (`BlueprintMapLibrary.Map_Find` _inactiveplayerwidgets _array_element))
    (`/Game/UI/InactivePlayerUI.UpdateBanners` _value)
    (`/Game/UI/InactivePlayerUI.UpdateCardCount` _value (`|GetArrayItem` (`self.Players`) _array_element))))

(fn `UserConstructionScript`)